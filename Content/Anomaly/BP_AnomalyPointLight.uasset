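; Point light actor for anomalies that can blink by flaring far above its default intensity.
; BeginPlay applies the default intensity, and a timeline's Update adds its track value, scaled by a very large multiplier, to that default.
; StartBlinking restarts the timeline from zero through direct component calls, while StopBlinking stops it and restores the default intensity.
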(event EventBeginPlay
  (Rendering|Components|Light|SetIntensity (Variables|Default|GetPointLight) (Variables|Default|GetDefaultIntensity)))

(fn ConstructionScript)

(fn StartBlinking
  (bind _blinktimeline (Variables|Default|GetBlinkTimeLine))
  (Audio|Components|Audio|Stop _blinktimeline)
  (Components|Timeline|SetPlaybackPosition _blinktimeline 0.0 false true)
  (Audio|Components|Audio|Play _blinktimeline))

(fn StopBlinking
  (Audio|Components|Audio|Stop (Variables|Default|GetBlinkTimeLine))
  (Rendering|Components|Light|SetIntensity (Variables|Default|GetPointLight) (Variables|Default|GetDefaultIntensity)))